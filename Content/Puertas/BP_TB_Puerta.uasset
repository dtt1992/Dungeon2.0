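; BP_TB_Puerta is a door that moves for BP_IronMan1 and also triggers enemy spawning.
; Overlapping the door box drives the mesh's Z through a timeline, whose update also starts a delay leading to a second timeline that sets the mesh location.
; A second box calls SpawnEnemigos on every BP_Spawn_Enemigos, then destroys both triggers and clears their flags, so the door cannot be triggered again.
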(event OnComponentBeginOverlap(BC_Puerta)
  (params (OverlappedComponent :type Primitive%20Component%20Object%20Reference) (OtherActor :type Actor%20Object%20Reference) (OtherComp :type Primitive%20Component%20Object%20Reference) (OtherBodyIndex :type Integer) (bFromSweep :type Boolean) (SweepResult :type Hit%20Result%20Structure%20%28by%20ref%29))
  (bind _sm_puerta (Variables|Default|GetSM_Puerta))
  (bind _sm_puerta_2 (Variables|Default|GetSM_Puerta))
  (bind _returnvalue (Transformation|GetWorldLocation _sm_puerta_2))
  (bind _returnvalue_2 (Transformation|GetWorldLocation _sm_puerta))
  (if (Variables|Default|GetPuerta_Abierta)
    (Utilities|Casting|CastToBP_IronMan1 OtherActor)
    (bind _newtrack_0 (Timeline|Movimiento_Puerta Play)
      (:Update
        (Transformation|SetWorldLocation _sm_puerta_2 (Math|Vector|MakeVector (.x _returnvalue) (.y _returnvalue) _newtrack_0) false false)
        (Utilities|FlowControl|Delay 6.0)
        (Timeline|Timeline_1 Play
          (:Update
            (Transformation|SetWorldLocation _sm_puerta (Math|Vector|MakeVector (.x _returnvalue_2) (.y _returnvalue_2) 0.0) false false)))))))

(event OnComponentBeginOverlap(BC_Activar_Enemigos)
  (params (OverlappedComponent :type Primitive%20Component%20Object%20Reference) (OtherActor :type Actor%20Object%20Reference) (OtherComp :type Primitive%20Component%20Object%20Reference) (OtherBodyIndex :type Integer) (bFromSweep :type Boolean) (SweepResult :type Hit%20Result%20Structure%20%28by%20ref%29))
  (if (Variables|Default|GetSpawn_Enemigos)
    (Utilities|Casting|CastToBP_IronMan1 OtherActor)
    (Development|PrintString "Hello" true true "(R=0.000000,G=0.660000,B=1.000000,A=1.000000)" 1e+01)
    (bind _outactors (Actor|GetAllActorsOfClass "/Game/P_Enemigos/Spawn_Enemigos/BP_Spawn_Enemigos.BP_Spawn_Enemigos_C"))
    (for _array_element _outactors
      (Default|SpawnEnemigos _array_element)
      (Collision|SetCollisionEnabled (Variables|Default|GetBC_Puerta) "NoCollision")
      (Components|DestroyComponent (Variables|Default|GetBC_Activar_Enemigos))
      (Variables|Default|SetSpawn_Enemigos false)
      (Components|DestroyComponent (Variables|Default|GetBC_Puerta))
      (Variables|Default|SetPuerta_Abierta false))))

(fn ConstructionScript)