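; Fire projectile for Iron Man that damages BP_Araña, BP_FrostGiant_Captain or BP_Thanos_1 on impact.
; Lanzar launches the Sphere with a velocity-change impulse along the given direction and places BolaFuego at the sphere's location.
; BeginPlay caches the BP_IronMan1 reference, whose Ataque value sets the damage.
; On hit, separate casts call each enemy's RestarVida and RecibirDaño, then the projectile destroys itself whatever it struck.
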(event OnComponentHit(Sphere)
  (params (HitComponent :type Primitive%20Component%20Object%20Reference) (OtherActor :type Actor%20Object%20Reference) (OtherComp :type Primitive%20Component%20Object%20Reference) (NormalImpulse :type Vector :default "0, 0, 0") (Hit :type Hit%20Result%20Structure%20%28by%20ref%29))
  (bind _ref_ironman (Variables|Default|GetRef_IronMan))
  (bind _ataque (Variables|/Game/P_Protagonista/IronMan/BP_IronMan1.BP_IronMan1_C|GetAtaque _ref_ironman))
  ;[1 1 1] Destruir el proyectil cuando impacte con cualquier cosa
  (Utilities|FlowControl|Sequence
    (:then_0
      (bind _asbp_araña (Utilities|Casting|CastToBP_Araña OtherActor))
      (Default|RestarVida _asbp_araña (Variables|/Game/P_Protagonista/IronMan/BP_IronMan1.BP_IronMan1_C|GetAtaque (Variables|Default|GetRef_IronMan)))
      (Default|RecibirDaño _asbp_araña Hit))
    (:then_1
      (bind _asbp_frost_giant_captain (Utilities|Casting|CastToBP_FrostGiant_Captain OtherActor))
      (Default|RestarVida _asbp_frost_giant_captain _ataque)
      (Default|RecibirDaño _asbp_frost_giant_captain Hit))
    (:then_2
      (bind _asbp_thanos_1 (Utilities|Casting|CastToBP_Thanos_1 OtherActor))
      (Default|RestarVida _asbp_thanos_1 _ataque)
      (Default|RecibirDaño _asbp_thanos_1 Hit))
    (:then_3
      (Actor|DestroyActor))))

(event Custom|Lanzar
  (params (Direccion :type Vector))
  (bind _sphere (Variables|Default|GetSphere))
  ;[1 1 1] Evento Lanzar el proyectil
  (Physics|AddImpulse _sphere (* Direccion (Variables|Default|GetVelocidad)) "None" true)
  (Transformation|SetWorldTransform (Variables|Default|GetBola_Fuego) (Math|Transform|MakeTransform (Transformation|GetWorldLocation _sphere) "0.000000,100.000000,0.000000" "1,1,1") false false))

(event EventBeginPlay
  (bind _outactors (Actor|GetAllActorsOfClass "/Game/P_Protagonista/IronMan/BP_IronMan1.BP_IronMan1_C"))
  (for _array_element _outactors
    (Variables|Default|SetRef_IronMan _array_element)))

(fn ConstructionScript)