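; BP_Proyectil_Fuego is a fireball projectile, filed under Iron Man's attacks, that damages certain enemies on impact.
; Lanzar launches the Sphere with a velocity-change impulse along the given direction scaled by Velocidad, then sets BolaFuego to the sphere's location with a fixed rotation.
; On hit, it passes the hit to RecibirDaño on BP_Enemigo3 or BP_FrostGiant_Captain, then destroys itself whatever it struck.
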(event OnComponentHit(Sphere)
  (params (HitComponent :type Primitive%20Component%20Object%20Reference) (OtherActor :type Actor%20Object%20Reference) (OtherComp :type Primitive%20Component%20Object%20Reference) (NormalImpulse :type Vector :default "0, 0, 0") (Hit :type Hit%20Result%20Structure%20%28by%20ref%29))
  ;[1 1 1] Destruir el proyectil cuando impacte con cualquier cosa
  (Utilities|FlowControl|Sequence
    (:then_0
      (bind _asbp_enemigo_3 (Utilities|Casting|CastToBP_Enemigo3 OtherActor))
      (Default|RecibirDaño _asbp_enemigo_3 Hit))
    (:then_1
      (bind _asbp_frost_giant_captain (Utilities|Casting|CastToBP_FrostGiant_Captain OtherActor))
      (Default|RecibirDaño _asbp_frost_giant_captain Hit))
    (:then_2
      (Actor|DestroyActor))))

(event Custom|Lanzar
  (params (Direccion :type Vector))
  (bind _sphere (Variables|Default|GetSphere))
  ;[1 1 1] Evento Lanzar el proyectil
  (Physics|AddImpulse _sphere (* Direccion (Variables|Default|GetVelocidad)) "None" true)
  (Transformation|SetWorldTransform (Variables|Default|GetBola_Fuego) (Math|Transform|MakeTransform (Transformation|GetWorldLocation _sphere) "0.000000,100.000000,0.000000" "1,1,1") false false))

(fn ConstructionScript)