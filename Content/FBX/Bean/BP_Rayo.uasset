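; BP_Rayo is a beam effect actor that links the Thanos character to the Iron Man character.
; BeginPlay caches references to BP_Thanos_1 and BP_IronMan1 through nested actor searches.
; The Lanzar_Rayo event loops over the Rayo particle component's instance parameters, assigning Thanos as "BeamSource" and Iron Man as "BeanTarget".
; It also sets emitter 1's beam target point to Iron Man's mesh location.
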(event Custom|Lanzar_Rayo
  (bind _rayo (Variables|Default|GetRayo))
  (for (_array_element _array_index) (Variables|/Script/Engine.ParticleSystemComponent|GetInstanceParameters _rayo)
    (switch int _array_index
      (:0
        (Utilities|Struct|SetmembersinParticleSysParam _array_element "BeamSource" "PSPT_Actor" (Variables|Default|GetRef_Thanos)))
      (:1
        (Class|ParticleSystemComponent|SetBeamTargetPoint _rayo 1 (Transformation|GetWorldLocation (Variables|/Script/Engine.Character|GetMesh (Variables|Default|GetRef_IronMan))) 1)
        (Utilities|Struct|SetmembersinParticleSysParam _array_element "BeanTarget" "PSPT_Actor" (Variables|Default|GetRef_IronMan))))))

(event EventBeginPlay
  (bind _outactors (Actor|GetAllActorsOfClass "/Game/BOSS/BP_Thanos_1.BP_Thanos_1_C"))
  (for _array_element _outactors
    (Variables|Default|SetRef_Thanos _array_element)
    (bind _outactors_2 (Actor|GetAllActorsOfClass "/Game/P_Protagonista/IronMan/BP_IronMan1.BP_IronMan1_C"))
    (for _array_element_2 _outactors_2
      (Variables|Default|SetRef_IronMan _array_element_2))))

(fn ConstructionScript)