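; Fire projectile actor that damages BP_IronMan1 on overlap, using the attack stat of BP_Thanos_1.
; BeginPlay caches a Thanos reference via GetAllActorsOfClass, keeping the last one found.
; Lanzar applies a velocity-change impulse along the given direction and sets the fire component's transform once at the projectile's location.
; Any overlap destroys the projectile; Iron Man first loses health by Thanos's Ataque and receives a Damage call.
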(event OnComponentBeginOverlap(ProyectilFuego)
  (params (OverlappedComponent :type Primitive%20Component%20Object%20Reference) (OtherActor :type Actor%20Object%20Reference) (OtherComp :type Primitive%20Component%20Object%20Reference) (OtherBodyIndex :type Integer) (bFromSweep :type Boolean) (SweepResult :type Hit%20Result%20Structure%20%28by%20ref%29))
  (Utilities|FlowControl|Sequence
    (:then_0
      (bind _asbp_iron_man_1 (Utilities|Casting|CastToBP_IronMan1 OtherActor))
      (Default|RestarVida _asbp_iron_man_1 (Variables|/Game/BOSS/BP_Thanos_1.BP_Thanos_1_C|GetAtaque (Variables|Default|GetRef.Thanos)))
      (Default|Damage _asbp_iron_man_1 0.0))
    (:then_1
      (Actor|DestroyActor))))

(event Custom|Lanzar
  (params (Direccion :type Vector))
  (bind _proyectilfuego (Variables|Default|GetProyectilFuego))
  (Physics|AddImpulse _proyectilfuego (* Direccion (Variables|Default|GetVelocidad)) "None" true)
  (Transformation|SetWorldTransform (Variables|Default|GetFuego) (Math|Transform|MakeTransform (Transformation|GetWorldLocation _proyectilfuego) "0.000000,100.000000,0.000000" "1,1,1") false false))

(event EventBeginPlay
  (bind _outactors (Actor|GetAllActorsOfClass "/Game/BOSS/BP_Thanos_1.BP_Thanos_1_C"))
  (for _array_element _outactors
    (Variables|Default|SetRef.Thanos _array_element)))

(fn ConstructionScript)