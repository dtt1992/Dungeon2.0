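; Child door Blueprint that spawns what its naming indicates is a key (llave) once its enemy count reaches zero.
; Tick polls the count while key creation is enabled and uses a DoOnce to trigger the spawn a single time.
; The construction script runs the parent's, then sizes and positions a box from variables.
; The spawn adds a child actor component at a random point inside that box.
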(event EventTick
  (params (DeltaSeconds :type Float%20%28single-precision%29))
  (if (Variables|Default|GetCrear_Llave)
    (if (<= (Variables|Default|GetEnemigos) 0)
      (Utilities|FlowControl|DoOnce false
        (:Completed
          (CallFunction|SpawnLlave0))))))

(fn ConstructionScript
  (|CallParentFunction)
  (Components|Box|SetBoxExtent (Variables|Default|GetBox_Llave_0) (Variables|Default|GetBox_Extent_Llave_0) true)
  (Transformation|SetRelativeLocation (Variables|Default|GetBox_Llave_0) (Variables|Default|GetSpawn_Posicion_Llave) false false))

(fn SpawnLlave0
  (bind _box_llave_0 (Variables|Default|GetBox_Llave_0))
  (AddComponent|AddChildActorComponent false (Math|Transform|MakeTransform (Math|Random|RandomPointinBoundingBox (Variables|/Script/Engine.SceneComponent|GetRelativeLocation _box_llave_0) (Variables|/Script/Engine.BoxComponent|GetBoxExtent _box_llave_0)) "0, 0, 0" "1,1,1")))