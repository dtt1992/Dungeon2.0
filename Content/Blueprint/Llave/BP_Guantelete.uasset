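; Gauntlet key pickup that lets BP_IronMan1 obtain the key for the final door.
; Plays a 2D sound on BeginPlay and pitches the gauntlet every tick by a frame-rate-dependent step while it exists.
; Overlap with Coger_Llave destroys only the gauntlet component, then sets TienesLlave on every BP_TB_Puerta_Final.
; The W_Tengo_Llave widget is created inside that loop, so one appears per door.
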(event OnComponentBeginOverlap(Coger_Llave)
  (params (OverlappedComponent :type Primitive%20Component%20Object%20Reference) (OtherActor :type Actor%20Object%20Reference) (OtherComp :type Primitive%20Component%20Object%20Reference) (OtherBodyIndex :type Integer) (bFromSweep :type Boolean) (SweepResult :type Hit%20Result%20Structure%20%28by%20ref%29))
  (bind _guantelete (Variables|Default|GetGuantelete))
  (Utilities|Casting|CastToBP_IronMan1 OtherActor)
  (Utilities|IsValid _guantelete
    (:Is%20Valid
      (Components|DestroyComponent _guantelete)
      (Variables|Default|SetExiste_Llave false)
      (bind _outactors (Actor|GetAllActorsOfClass "/Game/Blueprint/Puertas/BP_TB_Puerta_Final.BP_TB_Puerta_Final_C"))
      (for _array_element _outactors
        (Variables|/Game/Blueprint/Puertas/BP_TB_Puerta_Final.BP_TB_Puerta_Final_C|SetTienes_Llave? _array_element true)
        (bind _returnvalue (UserInterface|CreateWidget "/Game/Blueprint/Widget/W_Tengo_Llave.W_Tengo_Llave_C"))
        (UserInterface|Viewport|AddtoViewport _returnvalue 0)))))

(event EventBeginPlay
  (Audio|PlaySound2D "/Game/Musica/CE_Llave.CE_Llave"))

(event EventTick
  (params (DeltaSeconds :type Float%20%28single-precision%29))
  (if (Variables|Default|GetExiste_Llave)
    (Transformation|AddLocalRotation (Variables|Default|GetGuantelete) (Math|Rotator|MakeRotator 0.0 (+ DeltaSeconds 2.0) 0.0) false false)))

(fn ConstructionScript)