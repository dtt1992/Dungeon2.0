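; Door encounter actor that lifts a door for Iron Man, spawns enemies and keeps walls up until the enemy count reaches zero.
; An activation trigger spawns a random batch of alternating child actors inside a box and disables the door trigger.
; Blocking triggers destroy the walls at zero count, and the third also raises the door permanently via timeline.
; Construction script places triggers and spawn boxes from variables; key spawning is defined but uncalled here.
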(event OnComponentBeginOverlap(BC_Puerta)
  (params (OverlappedComponent :type Primitive%20Component%20Object%20Reference) (OtherActor :type Actor%20Object%20Reference) (OtherComp :type Primitive%20Component%20Object%20Reference) (OtherBodyIndex :type Integer) (bFromSweep :type Boolean) (SweepResult :type Hit%20Result%20Structure%20%28by%20ref%29))
  (bind _sm_puerta (Variables|Default|GetSM_Puerta))
  (bind _sm_puerta_2 (Variables|Default|GetSM_Puerta))
  (bind _returnvalue (Transformation|GetWorldLocation _sm_puerta))
  (bind _returnvalue_2 (Transformation|GetWorldLocation _sm_puerta_2))
  ;[1 1 1] Apertura Puerta
  (if (Variables|Default|GetPuerta_Abierta)
    (Utilities|Casting|CastToBP_IronMan1 OtherActor)
    (bind _newtrack_0 (Timeline|Movimiento_Puerta Play)
      (:Update
        (Transformation|SetWorldLocation _sm_puerta_2 (Math|Vector|MakeVector (.x _returnvalue_2) (.y _returnvalue_2) _newtrack_0) false false)
        (if (not (Variables|Default|GetSpawn_Enemigos))
          (Collision|SetCollisionEnabled (Variables|Default|GetMuro_3) "QueryAndPhysics")
          (Utilities|FlowControl|Delay 1.0)
          (Timeline|Timeline_1 Play
            (:Update
              (Transformation|SetWorldLocation _sm_puerta (Math|Vector|MakeVector (.x _returnvalue) (.y _returnvalue) 0.0) false false))))))))

(event OnComponentBeginOverlap(Puerta_Bloqueada_1)
  (params (OverlappedComponent :type Primitive%20Component%20Object%20Reference) (OtherActor :type Actor%20Object%20Reference) (OtherComp :type Primitive%20Component%20Object%20Reference) (OtherBodyIndex :type Integer) (bFromSweep :type Boolean) (SweepResult :type Hit%20Result%20Structure%20%28by%20ref%29))
  ;[1 1 1] Revision y bloqueo Puerta
  (if (<= (Variables|Default|GetEnemigos) 0)
    (if (Variables|Default|GetExiste_Muro)
      (Components|DestroyComponent (Variables|Default|GetMuro_1))
      (Components|DestroyComponent (Variables|Default|GetMuro_2))
      (Components|DestroyComponent (Variables|Default|GetMuro_3))
      (Variables|Default|SetExiste_Muro false))))

(event OnComponentBeginOverlap(Puerta_Bloqueada_2)
  (params (OverlappedComponent :type Primitive%20Component%20Object%20Reference) (OtherActor :type Actor%20Object%20Reference) (OtherComp :type Primitive%20Component%20Object%20Reference) (OtherBodyIndex :type Integer) (bFromSweep :type Boolean) (SweepResult :type Hit%20Result%20Structure%20%28by%20ref%29))
  ;[1 1 1] Revision y bloqueo Puerta 2
  (if (<= (Variables|Default|GetEnemigos) 0)
    (if (Variables|Default|GetExiste_Muro)
      (Components|DestroyComponent (Variables|Default|GetMuro_1))
      (Components|DestroyComponent (Variables|Default|GetMuro_2))
      (Components|DestroyComponent (Variables|Default|GetMuro_3))
      (Variables|Default|SetExiste_Muro false))))

(event OnComponentBeginOverlap(Auto_Puerta_Bloqueada_3)
  (params (OverlappedComponent :type Primitive%20Component%20Object%20Reference) (OtherActor :type Actor%20Object%20Reference) (OtherComp :type Primitive%20Component%20Object%20Reference) (OtherBodyIndex :type Integer) (bFromSweep :type Boolean) (SweepResult :type Hit%20Result%20Structure%20%28by%20ref%29))
  (bind _sm_puerta (Variables|Default|GetSM_Puerta))
  (bind _returnvalue (Transformation|GetWorldLocation _sm_puerta))
  ;[1 1 1] Revision y bloqueo Puerta 3
  (if (<= (Variables|Default|GetEnemigos) 0)
    (if (Variables|Default|GetExiste_Muro)
      (Components|DestroyComponent (Variables|Default|GetMuro_3))
      (Components|DestroyComponent (Variables|Default|GetAuto_Puerta_Bloqueada_3))
      (Components|DestroyComponent (Variables|Default|GetMuro_1))
      (Components|DestroyComponent (Variables|Default|GetMuro_2))
      (Variables|Default|SetExiste_Muro false)
      (bind _newtrack_0 (Timeline|Subir_Puerta_Permanente Play)
        (:Update
          (Transformation|SetWorldLocation _sm_puerta (Math|Vector|MakeVector (.x _returnvalue) (.y _returnvalue) _newtrack_0) false false))))))

(event OnComponentBeginOverlap(BC_Activar_Enemigos)
  (params (OverlappedComponent :type Primitive%20Component%20Object%20Reference) (OtherActor :type Actor%20Object%20Reference) (OtherComp :type Primitive%20Component%20Object%20Reference) (OtherBodyIndex :type Integer) (bFromSweep :type Boolean) (SweepResult :type Hit%20Result%20Structure%20%28by%20ref%29))
  ;[1 1 1] Creacion enemigos
  (if (Variables|Default|GetSpawn_Enemigos)
    (Utilities|Casting|CastToBP_IronMan1 OtherActor)
    (CallFunction|Spanw)
    (Collision|SetCollisionEnabled (Variables|Default|GetBC_Puerta) "NoCollision")
    (Components|DestroyComponent (Variables|Default|GetBC_Activar_Enemigos))
    (Variables|Default|SetSpawn_Enemigos false)
    (Components|DestroyComponent (Variables|Default|GetBC_Puerta))
    (Variables|Default|SetPuerta_Abierta false)))

(event EventTick
  (params (DeltaSeconds :type Float%20%28single-precision%29))
  ;[1 0.0658 0.03595] Test Verificar Contador enemigo
)

(fn ConstructionScript
  (Transformation|SetRelativeLocationAndRotation (Variables|Default|GetPuerta_Bloqueada_1) (Variables|Default|GetBloqueo_Puerta_1) (Math|Rotator|MakeRotator 0.0 0.0 (Variables|Default|GetGiro_Bloqueo_1)) false false)
  (Transformation|SetRelativeLocationAndRotation (Variables|Default|GetPuerta_Bloqueada_2) (Variables|Default|GetBloqueo_Puerta_2) (Math|Rotator|MakeRotator 0.0 0.0 (Variables|Default|GetGiro_Bloqueo_2)) false false)
  (Transformation|SetRelativeLocationAndRotation (Variables|Default|GetAuto_Puerta_Bloqueada_3) (Variables|Default|GetAuto_Bloqueo_Puerta_3) (Math|Rotator|MakeRotator 0.0 0.0 (Variables|Default|GetAuto_Giro_Bloqueo_3)) false false)
  (Transformation|SetRelativeLocation (Variables|Default|GetBox) (Variables|Default|GetSpawn_Enemy_Position) false false)
  (Components|Box|SetBoxExtent (Variables|Default|GetBox) (Variables|Default|GetBox_Extent) true)
  (Transformation|SetRelativeLocation (Variables|Default|GetBox_Llave) (Variables|Default|GetSpawn_Posicion_Llave) false false)
  (Components|Box|SetBoxExtent (Variables|Default|GetBox_Llave) (Variables|Default|GetBox_Extent_Llave) true))

(fn Spanw
  (bind _box (Variables|Default|GetBox))
  (bind _box_2 (Variables|Default|GetBox))
  (bind _boxextent (Variables|/Script/Engine.BoxComponent|GetBoxExtent _box_2))
  (bind _relativelocation (Variables|/Script/Engine.SceneComponent|GetRelativeLocation _box))
  (bind _returnvalue (Math|Random|RandomPointinBoundingBox _relativelocation _boxextent))
  (for _index (range 2 (Math|Random|RandomInteger 7))
    (Variables|Default|SetEnemigos _index)
    (Utilities|FlowControl|FlipFlop
      (:A
        (AddComponent|AddChildActorComponent false (Math|Transform|MakeTransform _returnvalue "0, 0, 0" "1,1,1")))
      (:B
        (AddComponent|AddChildActorComponent false (Math|Transform|MakeTransform _returnvalue "0, 0, 0" "1,1,1"))))))

(fn SpawnLlave
  (for _index (range 1 1)
    (AddComponent|AddChildActorComponent false (Math|Transform|MakeTransform (Math|Random|RandomPointinBoundingBox (Variables|/Script/Engine.SceneComponent|GetRelativeLocation (Variables|Default|GetBox_Llave)) (Variables|/Script/Engine.BoxComponent|GetBoxExtent (Variables|Default|GetBox_Llave))) "0, 0, 0" "1,1,1"))))