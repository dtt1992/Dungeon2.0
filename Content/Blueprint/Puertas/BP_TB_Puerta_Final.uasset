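; BP_TB_Puerta_Final is a final-door actor combining a timeline-driven sliding door, an enemy spawn trigger and a key-locked wall.
; BP_IronMan1 overlaps open the door, or spawn a child actor randomly inside a configurable box, briefly freezing the player and disabling door triggers.
; A separate trigger removes the wall if TienesLlave is set, otherwise shows a temporary key widget.
; Tick prints the enemy counter for debugging; Thanos health-widget creation is unconnected.
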(event OnComponentBeginOverlap(BC_Puerta)
  (params (OverlappedComponent :type Primitive%20Component%20Object%20Reference) (OtherActor :type Actor%20Object%20Reference) (OtherComp :type Primitive%20Component%20Object%20Reference) (OtherBodyIndex :type Integer) (bFromSweep :type Boolean) (SweepResult :type Hit%20Result%20Structure%20%28by%20ref%29))
  (bind _sm_puerta (Variables|Default|GetSM_Puerta))
  (bind _sm_puerta_2 (Variables|Default|GetSM_Puerta))
  (bind _returnvalue (Transformation|GetWorldLocation _sm_puerta))
  (bind _returnvalue_2 (Transformation|GetWorldLocation _sm_puerta_2))
  ;[1 1 1] Apertura Puerta
  (if (Variables|Default|GetPuerta_Abierta)
    (Utilities|Casting|CastToBP_IronMan1 OtherActor)
    (bind _newtrack_0 (Timeline|Movimiento_Puerta Play)
      (:Update
        (Transformation|SetWorldLocation _sm_puerta_2 (Math|Vector|MakeVector (.x _returnvalue_2) (.y _returnvalue_2) _newtrack_0) false false)
        (if (not (Variables|Default|GetSpawn_Enemigos))
          (Utilities|FlowControl|Delay 1.0)
          (Timeline|Timeline_1 Play
            (:Update
              (Transformation|SetWorldLocation _sm_puerta (Math|Vector|MakeVector (.x _returnvalue) (.y _returnvalue) 0.0) false false))))))))

(event OnComponentBeginOverlap(Puerta_Bloqueada_1)
  (params (OverlappedComponent :type Primitive%20Component%20Object%20Reference) (OtherActor :type Actor%20Object%20Reference) (OtherComp :type Primitive%20Component%20Object%20Reference) (OtherBodyIndex :type Integer) (bFromSweep :type Boolean) (SweepResult :type Hit%20Result%20Structure%20%28by%20ref%29))
  ;[1 1 1] Revision y bloqueo Puerta
  (Utilities|Casting|CastToBP_IronMan1 OtherActor)
  (if (Variables|Default|GetTienes_Llave?)
    (if (Variables|Default|GetExiste_Muro)
      (Components|DestroyComponent (Variables|Default|GetMuro_1))
      (Variables|Default|SetExiste_Muro false))
    (else
      (bind _returnvalue (UserInterface|CreateWidget "/Game/Blueprint/Widget/W_Llave.W_Llave_C"))
      (UserInterface|Viewport|AddtoViewport _returnvalue 0)
      (Utilities|FlowControl|Delay 5.0)
      (Widget|SetVisibility _returnvalue "Hidden"))))

(event OnComponentBeginOverlap(BC_Activar_Enemigos)
  (params (OverlappedComponent :type Primitive%20Component%20Object%20Reference) (OtherActor :type Actor%20Object%20Reference) (OtherComp :type Primitive%20Component%20Object%20Reference) (OtherBodyIndex :type Integer) (bFromSweep :type Boolean) (SweepResult :type Hit%20Result%20Structure%20%28by%20ref%29))
  ;[1 1 1] Creacion enemigos
  (bind _asbp_iron_man_1 (Utilities|Casting|CastToBP_IronMan1 OtherActor))
  (if (Variables|Default|GetSpawn_Enemigos)
    (CallFunction|Spawn)
    (Variables|/Script/Engine.CharacterMovementComponent|SetMaxWalkSpeed (Variables|/Script/Engine.Character|GetCharacterMovement _asbp_iron_man_1) 0.0)
    (Utilities|FlowControl|Delay 1.5)
    (Variables|/Script/Engine.CharacterMovementComponent|SetMaxWalkSpeed (Variables|/Script/Engine.Character|GetCharacterMovement _asbp_iron_man_1) 6e+02)
    (Collision|SetCollisionEnabled (Variables|Default|GetBC_Puerta) "NoCollision")
    (Components|DestroyComponent (Variables|Default|GetBC_Activar_Enemigos))
    (Variables|Default|SetSpawn_Enemigos false)
    (Components|DestroyComponent (Variables|Default|GetBC_Puerta))
    (Variables|Default|SetPuerta_Abierta false)))

(event EventTick
  (params (DeltaSeconds :type Float%20%28single-precision%29))
  (bind _enemigos (Variables|Default|GetEnemigos))
  ;[1 0.0658 0.03595] Test Verificar Contador enemigo
  (Utilities|FlowControl|Delay 1.0)
  (if (Variables|Default|GetCuenta_Enemigos)
    (if (not (<= _enemigos 0))
      (Development|PrintString (Utilities|String|ToString(Integer) _enemigos)))))

(fn ConstructionScript
  (Transformation|SetRelativeLocationAndRotation (Variables|Default|GetPuerta_Bloqueada_1) (Variables|Default|GetBloqueo_Puerta_1) (Math|Rotator|MakeRotator 0.0 0.0 (Variables|Default|GetGiro_Bloqueo_1)) false false)
  (Transformation|SetRelativeLocation (Variables|Default|GetBox) (Variables|Default|GetSpawn_Enemy_Position) false false)
  (Components|Box|SetBoxExtent (Variables|Default|GetBox) (Variables|Default|GetBox_Extent) true))

(fn Spawn
  (Variables|Default|SetEnemigos 0)
  (AddComponent|AddChildActorComponent false (Math|Transform|MakeTransform (Math|Random|RandomPointinBoundingBox (Variables|/Script/Engine.SceneComponent|GetRelativeLocation (Variables|Default|GetBox)) (Variables|/Script/Engine.BoxComponent|GetBoxExtent (Variables|Default|GetBox))) "0, 0, 0" "1.200000,1.200000,1.200000")))