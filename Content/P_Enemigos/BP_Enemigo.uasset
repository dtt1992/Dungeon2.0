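; BP_Enemigo is an enemy Blueprint with a Random_Enemigos event, apparently meant to randomize enemy appearance.
; The event loops over BpEnemigos and calls SetSkeletalMesh on each mesh with pose reinitialization, but supplies no new mesh.
; Disconnected leftover nodes sketch a choice between Frost Giant Captain and Greater Spider meshes, by random index or enemy type, and never execute.
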(event Custom|Random_Enemigos
  (for _array_element (Variables|Default|Getbp_enemigos)
    (Class|SkinnedMeshComponent|SetSkeletalMesh (Variables|/Script/Engine.Character|GetMesh _array_element) 0 true)))

(fn ConstructionScript)