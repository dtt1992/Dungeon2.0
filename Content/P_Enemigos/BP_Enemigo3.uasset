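; Spider enemy character that wanders the navmesh and switches to a faster chase when PawnSensing sees Iron Man.
; A delayed Tick loop drives AIMoveTo, while capsule overlaps toggle the attack flag in AB_Araña.
; A hit ragdolls it with a radial impulse and decrements the enemy count on every BP_TB_PuertaTest door.
; Melee damage checks the Daño_Derecha overlap but only prints a message.
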(event OnSeePawn(PawnSensing)
  (params (Pawn :type Pawn%20Object%20Reference))
  ;[1 1 1] Para detectar al pawn
  (bind _asbp_iron_man_1 (Utilities|Casting|CastToBP_IronMan1 Pawn))
  (Variables|Default|SetRef_IronMan _asbp_iron_man_1)
  (Variables|Default|SetDe_Paseo? false))

(event OnComponentBeginOverlap(CapsuleComponent)
  (params (OverlappedComponent :type Primitive%20Component%20Object%20Reference) (OtherActor :type Actor%20Object%20Reference) (OtherComp :type Primitive%20Component%20Object%20Reference) (OtherBodyIndex :type Integer) (bFromSweep :type Boolean) (SweepResult :type Hit%20Result%20Structure%20%28by%20ref%29))
  ;[1 1 1] Hacer que ataque el enemigo
  (Utilities|Casting|CastToBP_IronMan1 OtherActor)
  (bind _asab_araña (Utilities|Casting|CastToAB_Araña (Components|SkeletalMesh|GetAnimInstance (Variables|Character|GetMesh))))
  (Variables|/Game/InfinityBladeAdversaries/Enemy/Enemy_Great_Spider/AB_Araña.AB_Araña_C|SetPuedo_Atacar? _asab_araña true))

(event OnComponentBeginOverlap(Daño_Derecha)
  (params (OverlappedComponent :type Primitive%20Component%20Object%20Reference) (OtherActor :type Actor%20Object%20Reference) (OtherComp :type Primitive%20Component%20Object%20Reference) (OtherBodyIndex :type Integer) (bFromSweep :type Boolean) (SweepResult :type Hit%20Result%20Structure%20%28by%20ref%29))
  ;[1 1 1] Controlar cuando ataque el enemigo
  (if (== OtherActor (Variables|Default|GetRef_IronMan))
    (Variables|Default|SetJugador_colision_Daño? true)))

(event OnComponentEndOverlap(Daño_Derecha)
  (params (OverlappedComponent :type Primitive%20Component%20Object%20Reference) (OtherActor :type Actor%20Object%20Reference) (OtherComp :type Primitive%20Component%20Object%20Reference) (OtherBodyIndex :type Integer))
  ;[1 1 1] Controlar cuando ataque el enemigo
  (if (== OtherActor (Variables|Default|GetRef_IronMan))
    (Variables|Default|SetJugador_colision_Daño? false)))

(event OnComponentEndOverlap(CapsuleComponent)
  (params (OverlappedComponent :type Primitive%20Component%20Object%20Reference) (OtherActor :type Actor%20Object%20Reference) (OtherComp :type Primitive%20Component%20Object%20Reference) (OtherBodyIndex :type Integer))
  (Utilities|Casting|CastToBP_IronMan1 OtherActor
    (:then
      _)
    (:CastFailed
      _))
  (bind _asab_araña (Utilities|Casting|CastToAB_Araña (Components|SkeletalMesh|GetAnimInstance (Variables|Character|GetMesh))))
  (Variables|/Game/InfinityBladeAdversaries/Enemy/Enemy_Great_Spider/AB_Araña.AB_Araña_C|SetPuedo_Atacar? _asab_araña false))

(event Custom|Reanudar%20movimeinto
  ;[1 1 1] Controlar cuando ataque el enemigo
  (Pawn|Components|CharacterMovement|SetMovementMode (Variables|Character|GetCharacterMovement) "MOVE_NavWalking" 0))

(event Custom|Hacer_Daño
  ;[1 1 1] Controlar cuando ataque el enemigo
  (if (Variables|Default|GetJugador_colision_Daño?)
    (Development|PrintString "Hacer Daño")))

(event Custom|Recibir_Daño
  (params (Proyectil_Hit :type Hit%20Result%20Structure))
  (bind _mesh (Variables|Character|GetMesh))
  ;[1 1 1] Evento Recibir Daño
  (Physics|SetSimulatePhysics _mesh true)
  (Collision|SetCollisionEnabled _mesh "PhysicsOnly")
  (Physics|AddRadialImpulse _mesh (.Location (Collision|BreakHitResult Proyectil_Hit)) 5e+02 1e+03 "RIF_Constant" true)
  (Pawn|Components|CharacterMovement|DisableMovement (Variables|Character|GetCharacterMovement))
  (Collision|SetCollisionEnabled (Variables|Collision|GetCapsuleComponent) "NoCollision")
  (bind _outactors (Actor|GetAllActorsOfClass "/Game/Blueprint/BP_TB_PuertaTest.BP_TB_PuertaTest_C"))
  (for _array_element _outactors
    (if (> (Variables|/Game/Blueprint/BP_TB_PuertaTest.BP_TB_PuertaTest_C|GetEnemigos _array_element) 0)
      (Variables|/Game/Blueprint/BP_TB_PuertaTest.BP_TB_PuertaTest_C|SetEnemigos _array_element (- (Variables|/Game/Blueprint/BP_TB_PuertaTest.BP_TB_PuertaTest_C|GetEnemigos _array_element) 1)))))

(event Custom|Perseguir
  ;[1 1 1] Mover inteligencia artificial
)

(event Custom|Patrullar
  ;[1 1 1] Mover inteligencia artificial
)

(event Custom|Parar%20movimiento
  ;[1 1 1] Controlar cuando ataque el enemigo
  (Pawn|Components|CharacterMovement|DisableMovement (Variables|Character|GetCharacterMovement)))

(event EventTick
  (params (DeltaSeconds :type Float%20%28single-precision%29))
  (bind _ref_ironman (Variables|Default|GetRef_IronMan))
  (bind _charactermovement (Variables|Character|GetCharacterMovement))
  ;[1 1 1] Mover inteligencia artificial
  (Utilities|FlowControl|Delay 1.0)
  (if (Variables|Default|GetDe_Paseo?)
    (Variables|/Script/Engine.CharacterMovementComponent|SetMaxWalkSpeed _charactermovement 1.5e+02)
    (Utilities|FlowControl|Delay 0.2)
    (AI|AIMoveTo self (.RandomLocation (Class|NavigationSystem|GetRandomPointinNavigableRadius (Class|NavigationSystem|GetNavigationSystem) (Transformation|GetActorLocation) 2e+03)) 0 5.0 false)
    (else
      (Variables|/Script/Engine.CharacterMovementComponent|SetMaxWalkSpeed _charactermovement 5e+02)
      (Utilities|IsValid _ref_ironman
        (:Is%20Valid
          (AI|AIMoveTo self "0, 0, 0" _ref_ironman 5.0 false))
        (:Is%20Not%20Valid
          (Variables|Default|SetDe_Paseo? true))))))

(event EventBeginPlay
  ;[1 1 1] Mover inteligencia artificial
  (Variables|Default|SetRef_IronMan (Game|Player|GetPlayerPawn 0)))

(fn ConstructionScript)