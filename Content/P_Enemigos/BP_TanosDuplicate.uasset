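; Thanos enemy character that wanders the navmesh until PawnSensing spots Iron Man, then runs after the player.
; Tick drives movement and plays a melee montage within attack range, while separate events apply punch damage and toggle movement.
; A struct array holds its stats and feeds a health bar widget.
; Timelines animate material spawn and death dissolves, and a depleted stat triggers death and decrements door enemy counters.
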(event OnSeePawn(PawnSensing)
  (params (Pawn :type Pawn%20Object%20Reference))
  ;[1 1 1] Para detectar al pawn
  (bind _asbp_iron_man_1 (Utilities|Casting|CastToBP_IronMan1 Pawn))
  (Variables|Default|SetRef_IronMan1 _asbp_iron_man_1)
  (Variables|Default|SetDe_Paseo? false))

(event OnComponentBeginOverlap(CapsuleComponent)
  (params (OverlappedComponent :type Primitive%20Component%20Object%20Reference) (OtherActor :type Actor%20Object%20Reference) (OtherComp :type Primitive%20Component%20Object%20Reference) (OtherBodyIndex :type Integer) (bFromSweep :type Boolean) (SweepResult :type Hit%20Result%20Structure%20%28by%20ref%29))
  ;[1 1 1] Hacer que ataque el enemigo
  (Utilities|Casting|CastToBP_IronMan1 OtherActor)
  (bind _asb_anim_thanos (Utilities|Casting|CastToB_Anim_Thanos (Components|SkeletalMesh|GetAnimInstance (Variables|Character|GetMesh))))
  (Variables|/Game/BOSS/B_Anim_Thanos.B_Anim_Thanos_C|SetAtaque? _asb_anim_thanos true))

(event OnComponentEndOverlap(CapsuleComponent)
  (params (OverlappedComponent :type Primitive%20Component%20Object%20Reference) (OtherActor :type Actor%20Object%20Reference) (OtherComp :type Primitive%20Component%20Object%20Reference) (OtherBodyIndex :type Integer))
  ;[1 1 1] Hacer que ataque el enemigo
  (Utilities|Casting|CastToBP_IronMan1 OtherActor)
  (bind _asb_anim_thanos (Utilities|Casting|CastToB_Anim_Thanos (Components|SkeletalMesh|GetAnimInstance (Variables|Character|GetMesh))))
  (Variables|/Game/BOSS/B_Anim_Thanos.B_Anim_Thanos_C|SetAtaque? _asb_anim_thanos true))

(event OnComponentBeginOverlap(Dano_Izquierda)
  (params (OverlappedComponent :type Primitive%20Component%20Object%20Reference) (OtherActor :type Actor%20Object%20Reference) (OtherComp :type Primitive%20Component%20Object%20Reference) (OtherBodyIndex :type Integer) (bFromSweep :type Boolean) (SweepResult :type Hit%20Result%20Structure%20%28by%20ref%29))
  ;[1 1 1] Controlar cuando ataque el enemigo
  (if (== OtherActor (Variables|Default|GetRef_IronMan))
    (Variables|Default|SetJugador_colision_Daño? true)))

(event OnComponentEndOverlap(Dano_Izquierda)
  (params (OverlappedComponent :type Primitive%20Component%20Object%20Reference) (OtherActor :type Actor%20Object%20Reference) (OtherComp :type Primitive%20Component%20Object%20Reference) (OtherBodyIndex :type Integer))
  ;[1 1 1] Controlar cuando ataque el enemigo
  (if (== OtherActor (Variables|Default|GetRef_IronMan))
    (Variables|Default|SetJugador_colision_Daño? false)))

(event Custom|Muerte
  (bind _mesh (Variables|Character|GetMesh))
  ;[1 1 1] Cambio de material por muerte
  (Components|DestroyComponent (Variables|Collision|GetCapsuleComponent))
  (bind _returnvalue (Rendering|Material|CreateDynamicMaterialInstance _mesh 0 "/Game/Colores/Disaparecer/Troll/CharM_Frost_GiantTest_Inst.CharM_Frost_GiantTest_Inst" :!class /Script/Engine.PrimitiveComponent))
  (bind _returnvalue_2 (Rendering|Material|CreateDynamicMaterialInstance _mesh 1 "/Game/Colores/Disaparecer/Troll/CharM_Frost_GiantTest_Inst.CharM_Frost_GiantTest_Inst" :!class /Script/Engine.PrimitiveComponent))
  (bind _dissolver (Timeline|Timeline_0 Play)
    (:Update
      (Rendering|Material|SetScalarParameterValue _returnvalue "Amounts" _dissolver :!class /Script/Engine.MaterialInstanceDynamic)
      (Utilities|FlowControl|Delay 1.4)
      (Utilities|FlowControl|DoOnce false
        (:Completed
          (Actor|DestroyActor))))))

(event Custom|Reanudar%20movimeinto
  ;[1 1 1] Controlar cuando ataque el enemigo
  (Pawn|Components|CharacterMovement|SetMovementMode (Variables|Character|GetCharacterMovement) "MOVE_NavWalking" 0))

(event Custom|Hacer_Daño
  (params (Puñetazo_Hit :type Hit%20Result%20Structure))
  ;[1 1 1] Controlar cuando ataque el enemigo
  (Default|RestarVida (Variables|Default|GetRef_IronMan1) (Variables|Default|GetAtaque))
  (Audio|PlaySound2D "/Game/Sonido/Punch.Punch"))

(event Custom|Restar_Vida
  (params (Daño :type Float%20%28single-precision%29))
  ;[1 1 1] Recibir Daño
  (CallFunction|ModificarValores Daño "NewEnumerator1" "NewEnumerator0")
  (bind _asw_barra_estado_frost_giant (Utilities|Casting|CastToW_Barra_Estado_FrostGiant (UserInterface|GetUserWidgetObject (Variables|Default|GetW_Salud))))
  (Default|ActualizarBarraVidaEnemigo _asw_barra_estado_frost_giant (Variables|Default|GetArray_Valores)))

(event Custom|Recibir_Daño
  (params (Proyectil_Hit :type Hit%20Result%20Structure))
  ;[1 1 1] Evento Recibir Daño
  (for _array_element (Variables|Default|GetArray_Valores)
    (if (<= (Utilities|Struct|BreakS_Valores_Personajes _array_element) 0.0)
      (CallFunction|Muerte)
      (bind _outactors (Actor|GetAllActorsOfClass "/Game/Blueprint/BP_TB_PuertaTest.BP_TB_PuertaTest_C"))
      (for _array_element_2 _outactors
        (if (> (Variables|/Game/Blueprint/BP_TB_PuertaTest.BP_TB_PuertaTest_C|GetEnemigos _array_element_2) 0)
          (Variables|/Game/Blueprint/BP_TB_PuertaTest.BP_TB_PuertaTest_C|SetEnemigos _array_element_2 (- (Variables|/Game/Blueprint/BP_TB_PuertaTest.BP_TB_PuertaTest_C|GetEnemigos _array_element_2) 1)))))))

(event Custom|Parar%20movimiento
  ;[1 1 1] Controlar cuando ataque el enemigo
  (Pawn|Components|CharacterMovement|DisableMovement (Variables|Character|GetCharacterMovement)))

(event EventTick
  (params (DeltaSeconds :type Float%20%28single-precision%29))
  (bind _ref_ironman (Variables|Default|GetRef_IronMan))
  (bind _charactermovement (Variables|Character|GetCharacterMovement))
  ;[1 1 1] Mover inteligencia artificial
  (Utilities|FlowControl|Sequence
    (:then_0
      (Utilities|FlowControl|Delay 1.0)
      (if (Variables|Default|GetDe_Paseo?)
        (Variables|/Script/Engine.CharacterMovementComponent|SetMaxWalkSpeed _charactermovement 1.5e+02)
        (Utilities|FlowControl|Delay 0.2)
        (AI|AIMoveTo self (.RandomLocation (Class|NavigationSystem|GetRandomPointinNavigableRadius (Class|NavigationSystem|GetNavigationSystem) (Transformation|GetActorLocation) 2e+03)) 0 5.0 false)
        (else
          (Variables|/Script/Engine.CharacterMovementComponent|SetMaxWalkSpeed _charactermovement 5e+02)
          (Utilities|IsValid _ref_ironman
            (:Is%20Valid
              (AI|AIMoveTo self "0, 0, 0" _ref_ironman 5.0 false))
            (:Is%20Not%20Valid
              (Variables|Default|SetDe_Paseo? true))))))
    (:then_1
      ;[1 1 1] Controlar el ataque mediante distancia
      (if (< (Transformation|GetDistanceTo (Variables|Default|GetRef_IronMan)) (Variables|Default|GetRango_Ataque))
        (if (not (Class|AnimInstance|IsAnyMontagePlaying (Components|SkeletalMesh|GetAnimInstance (Variables|Character|GetMesh))))
          (bind _notifyname (Animation|Montage|PlayMontage (Variables|Character|GetMesh) "/Game/InfinityBladeAdversaries/Enemy/Enemy_Frost_Giant/AM_Ataque_FG_Captain.AM_Ataque_FG_Captain")
            (:then
              (Physics|AddImpulse (Variables|Default|GetDano_Izquierda) "0, 0, 0" "None" false))
            (:OnNotifyBegin
              (if (Utilities|Name|Equal(Name) _notifyname "daño")
                (bind _returnvalue (Effects|SpawnEmitteratLocation "/Game/InfinityBladeEffects/Effects/FX_Mobile/ICE/combat/P_HeldCharge_Ice_02.P_HeldCharge_Ice_02" "0, 0, 0"))
                (Transformation|AttachComponentToComponent _returnvalue (Variables|Character|GetMesh) "daño_Izquierda" "KeepRelative" "KeepRelative" "KeepRelative" true)))))))))

(event EventBeginPlay
  (bind _array_valores (Variables|Default|GetArray_Valores))
  ;[1 1 1] Poner todos los valores por defecto con una array
  (Variables|Default|SetRef_IronMan (Game|Player|GetPlayerPawn 0))
  (for (_array_element _array_index) _array_valores
    (bind _structout (Utilities|Struct|SetmembersinS_Valores_Personajes _array_element (Utilities|Struct|BreakS_Valores_Personajes _array_element)))
    (Utilities|Array|SetArrayElem _array_valores _array_index _structout)
    (bind _returnvalue (Rendering|Material|CreateDynamicMaterialInstance (Variables|Character|GetMesh) 0 "/Game/Blueprint/Desvanecimiento/M_Material_Inst.M_Material_Inst" :!class /Script/Engine.PrimitiveComponent))
    (bind _aparicion (Timeline|Aparicion Play)
      (:Update
        (Rendering|Material|SetScalarParameterValue _returnvalue "Amount" _aparicion :!class /Script/Engine.MaterialInstanceDynamic)
        (Utilities|FlowControl|Delay 3.0)
        (Rendering|Material|SetMaterial (Variables|Character|GetMesh) 0 "/Game/BOSS/Pose_T/COC_iOS_VIL_THA_CUR_B.COC_iOS_VIL_THA_CUR_B")))))

(fn ConstructionScript)

(fn ModificarValores
  (params (Cantidad :type Float%20%28single-precision%29) (Operacion :type E_Tipos_Operaciones%20Enum :default "NewEnumerator0") (Tipo_Valor :type E_Tipos_Valores%20Enum :default "NewEnumerator0"))
  (LocalVariables|SetCantidad_Actual Cantidad)
  (bind _indice_tipo_valor (CallFunction|FuncionTipoValores Tipo_Valor))
  (switch Utilities|FlowControl|Switch|SwitchonE_Tipos_Operaciones Operacion
    (:NewEnumerator0
      (Utilities|Struct|SetmembersinS_Valores_Personajes (Utilities|Array|Get(acopy) (Variables|Default|GetArray_Valores) _indice_tipo_valor) (Math|Float|Clamp(Float) (+ (LocalVariables|GetCantidad_Actual) (.Valor_Actual (Utilities|Struct|BreakS_Valores_Personajes (Utilities|Array|Get(acopy) (Variables|Default|GetArray_Valores) _indice_tipo_valor)))) 0.0 (.Valor_Maximo (Utilities|Struct|BreakS_Valores_Personajes (Utilities|Array|Get(acopy) (Variables|Default|GetArray_Valores) _indice_tipo_valor))))))
    (:NewEnumerator1
      (Utilities|Struct|SetmembersinS_Valores_Personajes (Utilities|Array|Get(acopy) (Variables|Default|GetArray_Valores) _indice_tipo_valor) (Math|Float|Clamp(Float) (- (.Valor_Actual (Utilities|Struct|BreakS_Valores_Personajes (Utilities|Array|Get(acopy) (Variables|Default|GetArray_Valores) _indice_tipo_valor))) (LocalVariables|GetCantidad_Actual)) 0.0 (.Valor_Maximo (Utilities|Struct|BreakS_Valores_Personajes (Utilities|Array|Get(acopy) (Variables|Default|GetArray_Valores) _indice_tipo_valor))))))))

(fn FuncionTipoValores
  (params (Tipos_Valores :type E_Tipos_Valores%20Enum :default "NewEnumerator0"))
  (bind _array_valores (Variables|Default|GetArray_Valores))
  (for (_array_element _array_index) _array_valores
    (bind _structout (Utilities|Struct|SetmembersinS_Valores_Personajes _array_element Tipos_Valores))
    (if (!= (Utilities|Array|FindItem _array_valores _structout) -1)
      (return _array_index)))
  (return -1))