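; BP_Spawn_Enemigos is an enemy spawner actor that scatters child actors inside its Box component.
; SpawnEnemigos loops a random number of times, with a FlipFlop alternating between two AddChildActorComponent calls.
; Each child is placed at a random point in the box, then the box extent is set from BoxExtent.
; The SpawnEnemigos call in the construction script graph is disconnected and BeginPlay is empty, so nothing here triggers spawning.
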(event EventBeginPlay)

(fn ConstructionScript)

(fn SpawnEnemigos
  (bind _box (Variables|Default|GetBox))
  (bind _box_2 (Variables|Default|GetBox))
  (bind _boxextent (Variables|/Script/Engine.BoxComponent|GetBoxExtent _box_2))
  (bind _relativelocation (Variables|/Script/Engine.SceneComponent|GetRelativeLocation _box))
  (bind _returnvalue (Math|Random|RandomPointinBoundingBox _relativelocation _boxextent))
  (for _index (range 1 (Math|Random|RandomInteger 7))
    (Variables|Default|SetEnemigos _index)
    (Utilities|FlowControl|FlipFlop
      (:A
        (AddComponent|AddChildActorComponent false (Math|Transform|MakeTransform _returnvalue "0, 0, 0" "1,1,1"))
        (Components|Box|SetBoxExtent (Variables|Default|GetBox) (Variables|Default|GetBox_Extent) true))
      (:B
        (AddComponent|AddChildActorComponent false (Math|Transform|MakeTransform _returnvalue "0, 0, 0" "1,1,1"))
        (Components|Box|SetBoxExtent (Variables|Default|GetBox) (Variables|Default|GetBox_Extent) true)))))